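; BP_Enermy is an enemy character that takes damage, reacts to hits and dies.
; Any damage lowers HP through RHCharacterState and plays the AM_Damaged montage.
; When that state reports death, it triggers the death animation in ABP_RHCharacter, disables mesh and capsule collision, then destroys the actor after a delay.
; The death step runs only if the mesh's anim instance casts to ABP_RHCharacter.
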(event `self.ReceiveAnyDamage`
  (params (Damage :type "Float (single-precision)") (DamageType :type "DamageType Object Reference") (InstigatedBy :type "Controller Object Reference") (DamageCauser :type "Actor Object Reference"))
  (`RHCharacterState.DecreaseHP` (`self.RHCharacterState`) Damage)
  (`self.PlayAnimMontage` "/Game/Asset/RedHood/HuntCharacter/Animation/AM_Damaged.AM_Damaged")
  (if (`RHCharacterState.bIsDead` (`self.RHCharacterState`))
    (bind _asabp_rhcharacter (cast `/Game/BluePrint/Character/ABP_RHCharacter` (`SkeletalMeshComponent.GetAnimInstance` (`self.Mesh`))))
    (`/Game/BluePrint/Character/ABP_RHCharacter.AnimCharacterDead` _asabp_rhcharacter)
    (`self.Dead`)))

(event `Dead`
  (`PrimitiveComponent.SetCollisionEnabled` (`self.Mesh`) "NoCollision")
  (`PrimitiveComponent.SetCollisionEnabled` (`self.CapsuleComponent`) "NoCollision")
  (`KismetSystemLibrary.Delay` 7.0)
  (`self.K2_DestroyActor`))

(fn `UserConstructionScript`)