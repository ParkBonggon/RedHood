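; BP_CharacterState is a component that tracks health for its owning BP_RHCharacter.
; On BeginPlay it waits one tick, caches the owner, fills health to maximum and updates the HUD's health bar and text.
; DecreaseHP and IncreaseHP adjust health and refresh the HUD, with healing capped at maximum.
; At zero or below, DecreaseHP calls the death animation on the mesh's ABP_RHCharacter and returns true, even on repeated hits.
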(event `self.ReceiveBeginPlay`
  (`KismetSystemLibrary.DelayUntilNextTick`)
  (bind _asbp_rhcharacter (cast `/Game/BluePrint/Character/BP_RHCharacter` (`self.GetOwner`)))
  (bind _output_get (set `self.BP_Character` _asbp_rhcharacter))
  (bind _output_get_2 (set `self.CurrentHealth` (`self.MaxHealth`)))
  (bind _character_hud (`/Game/BluePrint/Character/BP_RHCharacter.Character HUD` _output_get))
  (`ProgressBar.SetPercent` (`/Game/BluePrint/Character/CharacterState/BP_CharacterHUD.HPBar` _character_hud) (/ _output_get_2 (`self.MaxHealth`)))
  (`TextBlock.SetText` (`/Game/BluePrint/Character/CharacterState/BP_CharacterHUD.HPPercent` _character_hud) (`KismetTextLibrary.Conv_DoubleToText` (`self.CurrentHealth`) "HalfToEven")))

(fn `Decrease HP`
  (params (Damage :type "Float (double-precision)"))
  (returns (bIsDead :type Boolean))
  (bind _character_hud (`/Game/BluePrint/Character/BP_RHCharacter.Character HUD` (`self.BP_Character`)))
  (if (not (<= (`self.CurrentHealth`) 0.0))
    (bind _output_get (set `self.CurrentHealth` (- (`self.CurrentHealth`) Damage)))
    (`ProgressBar.SetPercent` (`/Game/BluePrint/Character/CharacterState/BP_CharacterHUD.HPBar` _character_hud) (/ _output_get (`self.MaxHealth`)))
    (`TextBlock.SetText` (`/Game/BluePrint/Character/CharacterState/BP_CharacterHUD.HPPercent` _character_hud) (`KismetTextLibrary.Conv_DoubleToText` (`self.CurrentHealth`) "HalfToEven"))
    (if (<= (`self.CurrentHealth`) 0.0)
      _
      (else
        (return false))))
  (bind _asabp_rhcharacter (cast `/Game/BluePrint/Character/ABP_RHCharacter` (`SkeletalMeshComponent.GetAnimInstance` (`Character.Mesh` (`self.BP_Character`))))
    (:`then`
      (`/Game/BluePrint/Character/ABP_RHCharacter.AnimCharacterDead` _asabp_rhcharacter))
    (:`CastFailed`
      _))
  (return true))

(fn `Increase HP`
  (params (`Incerease HP` :type "Float (double-precision)"))
  (bind _character_hud (`/Game/BluePrint/Character/BP_RHCharacter.Character HUD` (`self.BP_Character`)))
  (bind _output_get (set `self.CurrentHealth` (+ `Incerease HP` (`self.CurrentHealth`))))
  (if (>= (`self.CurrentHealth`) (`self.MaxHealth`))
    (set `self.CurrentHealth` (`self.MaxHealth`)))
  (`ProgressBar.SetPercent` (`/Game/BluePrint/Character/CharacterState/BP_CharacterHUD.HPBar` _character_hud) (/ _output_get (`self.MaxHealth`)))
  (`TextBlock.SetText` (`/Game/BluePrint/Character/CharacterState/BP_CharacterHUD.HPPercent` _character_hud) (`KismetTextLibrary.Conv_DoubleToText` (`self.CurrentHealth`) "HalfToEven")))